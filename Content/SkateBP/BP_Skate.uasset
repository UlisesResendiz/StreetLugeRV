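; BP_Skate is the player-controlled skater, which moves forward constantly along the control rotation and steers through controller yaw from the MoveRight and MoveLeft axes.
; BeginPlay adds the GUI widget, and Tick converts velocity into a whole-number km/h string.
; A and D set left and right flags, which Tick copies to the BP_Character animation instance with per-side values that grow while held and reset on release.
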(event EventBeginPlay
  (bind _returnvalue (UserInterface|CreateWidget "/Game/SkateBP/GUI.GUI_C"))
  (UserInterface|Viewport|AddtoViewport _returnvalue 0))

(event Collision|EventActorBeginOverlap
  (params (OtherActor :type Actor%20Object%20Reference)))

(event EventTick
  (params (DeltaSeconds :type Float%20%28single-precision%29))
  (Utilities|FlowControl|Sequence
    (:then_0
      (Pawn|Input|AddMovementInput (Math|Vector|GetForwardVector (Pawn|GetControlRotation :!class /Script/Engine.Pawn)) 1.0 false)
      (bind _output_get (Variables|Default|SetVelocidad (Math|Vector|VectorLength (Transformation|GetVelocity))))
      (Variables|Default|SetPrintVelocidad (Utilities|String|ToString(Integer) (Math|Float|Floor (Math|Float|Absolute(Float) (* _output_get 0.036))))))
    (:then_1
      (bind _asbp_character (Utilities|Casting|CastToBP_Character (Components|SkeletalMesh|GetAnimInstance (Variables|Default|GetCharacter))))
      (Variables|Default|SetAnimation_Character _asbp_character))
    (:then_2
      (Variables|/Game/Models/Character/Animation/BP_Character.BP_Character_C|Setizq (Variables|Default|GetAnimation_Character) (Variables|Default|GetIsLeft?))
      (Variables|/Game/Models/Character/Animation/BP_Character.BP_Character_C|Setderr (Variables|Default|GetAnimation_Character) (Variables|Default|GetIsRight?)))
    (:then_3
      (if (Variables|Default|GetIsLeft?)
        (Variables|/Game/Models/Character/Animation/BP_Character.BP_Character_C|SetIzqValue (Variables|Default|GetAnimation_Character) (+ (Variables|/Game/Models/Character/Animation/BP_Character.BP_Character_C|GetIzqValue (Variables|Default|GetAnimation_Character)) 5.0))
        (else
          (Variables|/Game/Models/Character/Animation/BP_Character.BP_Character_C|SetIzqValue (Variables|Default|GetAnimation_Character) 0.0))))
    (:then_4
      (if (Variables|Default|GetIsRight?)
        (Variables|/Game/Models/Character/Animation/BP_Character.BP_Character_C|SetDerValue (Variables|Default|GetAnimation_Character) (+ (Variables|/Game/Models/Character/Animation/BP_Character.BP_Character_C|GetDerValue (Variables|Default|GetAnimation_Character)) 5.0))
        (else
          (Variables|/Game/Models/Character/Animation/BP_Character.BP_Character_C|SetDerValue (Variables|Default|GetAnimation_Character) 0.0))))))

(event Input|AxisEvents|InputAxisMoveRight
  (params (AxisValue :type Float%20%28single-precision%29))
  ;[1 1 1] Movimiento
  (Pawn|Input|AddControllerYawInput (* AxisValue 0.5)))

(event Input|AxisEvents|InputAxisMoveLeft
  (params (AxisValue :type Float%20%28single-precision%29))
  ;[1 1 1] Movimiento
  (Pawn|Input|AddControllerYawInput (* AxisValue 0.5)))

(event Input|KeyboardEvents|A
  (params (Key :type Key%20Structure :default "None"))
  ;[1 1 1] Movimiento
  (:Pressed
    (Variables|Default|SetIsLeft? true))
  (:Released
    (Variables|Default|SetIsLeft? false)))

(event Input|KeyboardEvents|D
  (params (Key :type Key%20Structure :default "None"))
  ;[1 1 1] Movimiento
  (:Pressed
    (Variables|Default|SetIsRight? true))
  (:Released
    (Variables|Default|SetIsRight? false)))

(fn ConstructionScript)